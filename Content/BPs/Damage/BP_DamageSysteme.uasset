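; Damage component that gives its owning actor a Life value and tags it "Damage".
; It binds to the owner's OnTakeAnyDamage, subtracts truncated damage through UpdateLife, then runs CheckDeath.
; CheckDeath destroys non-player owners at zero Life or below; for players it only returns the death state, which is unused here.
; For players, it also prints the yaw-only angle between facing and the damage causer's direction.
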(event Custom|ReceiveDamage
  (params (DamagedActor :type Actor%20Object%20Reference) (Damage :type Float%20%28single-precision%29) (DamageType :type Damage%20Type%20Object%20Reference) (InstigatedBy :type Controller%20Object%20Reference) (DamageCauser :type Actor%20Object%20Reference))
  (bind _returnvalue (Actor|ActorHasTag DamagedActor "Player"))
  (CallFunction|UpdateLife (Math|Float|Truncate Damage) false)
  (Utilities|FlowControl|Sequence
    (:then_0
      (CallFunction|CheckDeath _returnvalue))
    (:then_1
      (if _returnvalue
        (bind _angle (CallFunction|GetAngleBetweenVectors false (Math|Vector|GetForwardVector (Math|Rotator|MakeRotator 0.0 0.0 (.yaw (Transformation|GetWorldRotation (Variables|/Script/Engine.Actor|GetRootComponent DamagedActor))))) (Math|Vector|GetForwardVector (Math|Rotator|MakeRotator 0.0 0.0 (.yaw (Math|Rotator|FindLookatRotation (Transformation|GetWorldLocation (Variables|/Script/Engine.Actor|GetRootComponent DamagedActor)) (Transformation|GetWorldLocation (Variables|/Script/Engine.Actor|GetRootComponent DamageCauser))))))))
        (Development|PrintString (Utilities|String|ToString(Float) _angle))))))

(event EventBeginPlay
  (bind _returnvalue (Components|GetOwner))
  (Utilities|Array|AddUnique (Variables|/Script/Engine.Actor|GetTags _returnvalue) "Damage")
  (EventDispatchers|BindEventtoOnTakeAnyDamage _returnvalue (delegate Custom|ReceiveDamage)))

(fn UpdateLife
  (params (Value :type Integer) (Adding :type Boolean))
  (Variables|Default|SetLife (+ (Variables|Default|GetLife) (* Value (select Adding 1 -1)))))

(fn CheckDeath
  (params (IsPlayer :type Boolean))
  (if (and (not IsPlayer) (<= (Variables|Default|GetLife) 0))
    (Actor|DestroyActor (Components|GetOwner)))
  (return (and IsPlayer (<= (Variables|Default|GetLife) 0))))