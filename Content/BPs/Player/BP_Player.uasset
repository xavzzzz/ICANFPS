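; First-person player character with Enhanced Input move, look, jump, dash and slide.
; BeginPlay adds movement and shooting mapping contexts, then reads speed, jump height and dash distance from DT_Player.
; Dash capsule-traces a fixed distance along the last move direction, then timeline-lerps to the hit or endpoint.
; Slide briefly crouches, lowers the camera and boosts walk speed on the ground.
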(event Input|EnhancedActionEvents|EnhancedInputActionIA_Move
  (params (ActionValue :type Vector%202D%20Structure) (ElapsedSeconds :type Float%20%28double-precision%29) (TriggeredSeconds :type Float%20%28double-precision%29) (InputAction :type Input%20Action%20Object%20Reference :default "/Game/Inputs/Actions/Movement/IA_Move.IA_Move"))
  (bind _returnvalue (Transformation|GetActorForwardVector))
  (bind _returnvalue_2 (Transformation|GetActorRightVector))
  (:Triggered
    (Pawn|Input|AddMovementInput _returnvalue_2 (.x ActionValue) true)
    (Pawn|Input|AddMovementInput _returnvalue (.y ActionValue) true)
    (Variables|Default|SetDirection (+ (* _returnvalue_2 (.x ActionValue)) (* _returnvalue (.y ActionValue))))))

(event Input|EnhancedActionEvents|EnhancedInputActionIA_Look
  (params (ActionValue :type Vector%202D%20Structure) (ElapsedSeconds :type Float%20%28double-precision%29) (TriggeredSeconds :type Float%20%28double-precision%29) (InputAction :type Input%20Action%20Object%20Reference :default "/Game/Inputs/Actions/Movement/IA_Look.IA_Look"))
  (:Triggered
    (Pawn|Input|AddControllerYawInput (.x ActionValue))
    (Pawn|Input|AddControllerPitchInput (.y ActionValue))))

(event Input|EnhancedActionEvents|EnhancedInputActionIA_Dash
  (params (ActionValue :type Boolean) (ElapsedSeconds :type Float%20%28double-precision%29) (TriggeredSeconds :type Float%20%28double-precision%29) (InputAction :type Input%20Action%20Object%20Reference :default "/Game/Inputs/Actions/Movement/IA_Dash.IA_Dash"))
  (bind _self self)
  (bind _self_2 self)
  (bind _capsulecomponent (Variables|Collision|GetCapsuleComponent))
  (bind _returnvalue (Transformation|GetActorLocation _self))
  (bind _returnvalue_2 (Transformation|GetActorLocation _self_2))
  ;[0 0 0] Dash
  (:Started
    (if (Variables|Default|GetCanDash)
      (Variables|Default|SetCanDash false)
      (bind _outhit (Collision|CapsuleTraceByChannel _returnvalue_2 (+ _returnvalue_2 (* (Variables|Default|GetDirection) 5e+02)) (Variables|/Script/Engine.CapsuleComponent|GetCapsuleRadius _capsulecomponent) (Variables|/Script/Engine.CapsuleComponent|GetCapsuleHalfHeight _capsulecomponent) "TraceTypeQuery1" false 0 "Persistent"))
      (Variables|/Script/Engine.CharacterMovementComponent|SetMaxWalkSpeed (Variables|Character|GetCharacterMovement) 0.0)
      (bind _alpha (Timeline|Dash PlayFromStart)
        (:Update
          (Transformation|SetActorLocation self (Math|Vector|Lerp(Vector) (Math|Vector|MakeVector (.x _returnvalue) (.y _returnvalue) (.z _returnvalue)) (select (.bBlockingHit (Collision|BreakHitResult _outhit)) (Math|Vector|MakeVector (.x (.Location (Collision|BreakHitResult _outhit))) (.y (.Location (Collision|BreakHitResult _outhit))) (.z _returnvalue)) (Math|Vector|MakeVector (.x (.TraceEnd (Collision|BreakHitResult _outhit))) (.y (.TraceEnd (Collision|BreakHitResult _outhit))) (.z _returnvalue))) _alpha) false false)
          (Utilities|FlowControl|Delay 2.0)
          (Variables|Default|SetCanDash true))
        (:Finished
          (Variables|/Script/Engine.CharacterMovementComponent|SetMaxWalkSpeed (Variables|Character|GetCharacterMovement) (Variables|Default|GetMax%20Walk%20Speed)))))))

(event Input|EnhancedActionEvents|EnhancedInputActionIA_Slide
  (params (ActionValue :type Boolean) (ElapsedSeconds :type Float%20%28double-precision%29) (TriggeredSeconds :type Float%20%28double-precision%29) (InputAction :type Input%20Action%20Object%20Reference :default "/Game/Inputs/Actions/Movement/IA_Slide.IA_Slide"))
  (bind _charactermovement (Variables|Character|GetCharacterMovement))
  ;[0 0 0] Slide
  (:Started
    (Development|PrintString "SLIDE")
    (if (AI|Components|NavMovement|IsMovingonGround (Variables|Character|GetCharacterMovement))
      (Transformation|AddLocalOffset (Variables|Default|GetCamera) (Math|Vector|MakeVector 0.0 0.0 -2e+01) true false)
      (Character|Crouch)
      (bind _output_get (Variables|Default|SetMax%20Walk%20Speed (Variables|/Script/Engine.CharacterMovementComponent|GetMaxWalkSpeed _charactermovement)))
      (Variables|/Script/Engine.CharacterMovementComponent|SetMaxWalkSpeed _charactermovement (* _output_get 3.0))
      (Utilities|FlowControl|Delay 0.5)
      (Variables|/Script/Engine.CharacterMovementComponent|SetMaxWalkSpeed _charactermovement _output_get)
      (Transformation|AddLocalOffset (Variables|Default|GetCamera) (Math|Vector|MakeVector 0.0 0.0 2e+01) true false)
      (Character|UnCrouch))))

(event Input|EnhancedActionEvents|EnhancedInputActionIA_Crouch
  (params (ActionValue :type Boolean) (ElapsedSeconds :type Float%20%28double-precision%29) (TriggeredSeconds :type Float%20%28double-precision%29) (InputAction :type Input%20Action%20Object%20Reference :default "/Game/Inputs/Actions/Movement/IA_Crouch.IA_Crouch")))

(event Input|EnhancedActionEvents|EnhancedInputActionIA_Jump
  (params (ActionValue :type Boolean) (ElapsedSeconds :type Float%20%28double-precision%29) (TriggeredSeconds :type Float%20%28double-precision%29) (InputAction :type Input%20Action%20Object%20Reference :default "/Game/Inputs/Actions/Movement/IA_Jump.IA_Jump"))
  (:Started
    (if (Character|CanJump)
      (Character|Jump))))

(event EventBeginPlay
  (Utilities|FlowControl|Sequence
    (:then_0
      (CallFunction|SetupInput))
    (:then_1
      (CallFunction|SetupPlayerSettings))))

(fn ConstructionScript)

(fn SetupInput
  (bind _returnvalue (Game|GetPlayerController 0))
  (bind _returnvalue_2 (PlayerController|LocalPlayerSubsystems|GetEnhancedInputLocalPlayerSubsystem _returnvalue))
  (Utilities|IsValid _returnvalue_2
    (:Is%20Valid
      (Input|AddMappingContext _returnvalue_2 "/Game/Inputs/IM_FPSMovement.IM_FPSMovement" 0 "(bIgnoreAllPressedKeysUntilRelease=True,bForceImmediately=False)")
      (Input|AddMappingContext _returnvalue_2 "/Game/Inputs/IM_FPSShoot.IM_FPSShoot" 0 "(bIgnoreAllPressedKeysUntilRelease=True,bForceImmediately=False)"))))

(fn SetupPlayerSettings
  (bind _charactermovement (Variables|Character|GetCharacterMovement))
  (bind _returnvalue (Utilities|GetDataTableRow "/Game/Data/Tables/DT_Player.DT_Player" (Variables|Default|GetPlayerRowName))
    (:then
      (Utilities|FlowControl|Sequence
        (:then_0
          (Variables|/Script/Engine.CharacterMovementComponent|SetMaxWalkSpeed _charactermovement (.speed _returnvalue))
          (Development|PrintString "Speed is Ok"))
        (:then_1
          (bind _velocity (CallFunction|JumpVelocitybyHeight (.jumpheight _returnvalue) (Components|Movement|GetGravityZ (Variables|Character|GetCharacterMovement))))
          (bind _output_get (Variables|/Script/Engine.CharacterMovementComponent|SetJumpZVelocity _charactermovement _velocity))
          (Development|PrintString (Utilities|String|Append "Jump Heigt is Ok " (Utilities|String|ToString(Float) _output_get))))
        (:then_2
          (Variables|Default|SetDashSpeed (.dashdistance _returnvalue)))))))

(fn CalculeDashVector
  (bind _charactermovement (Variables|Character|GetCharacterMovement))
  (return (* (/ (Variables|/Script/Engine.MovementComponent|GetVelocity _charactermovement) (Variables|/Script/Engine.CharacterMovementComponent|GetMaxWalkSpeed _charactermovement)) (Variables|Default|GetDashSpeed))))